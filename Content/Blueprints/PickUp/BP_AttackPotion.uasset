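; BP_AttackPotion is a pickup potion that permanently raises the player character's attack power when used.
; OnUse adds the potion's Value to AttackPower on player 0's BP_ARPGCharacter, with no timer or reversal in this graph.
; The separate Extra event grants small fixed amounts of Money and Exp, then shows a WB_GetInfo widget fed with GetInfo.
; Neither event is triggered within this Blueprint.
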(event EventBeginPlay)

(event Collision|EventActorBeginOverlap
  (params (OtherActor :type Actor%20Object%20Reference)))

(event EventTick
  (params (DeltaSeconds :type Float%20%28single-precision%29)))

(event EventOnUse
  (bind _returnvalue (Game|GetPlayerCharacter 0))
  (bind _asbp_arpgcharacter (Utilities|Casting|CastToBP_ARPGCharacter _returnvalue))
  (Variables|/Script/Guaduation_ARPG.ARPGCharacter|SetAttackPower _asbp_arpgcharacter (+ (Variables|/Script/Guaduation_ARPG.ARPGCharacter|GetAttackPower _asbp_arpgcharacter) (Variables|Default|GetValue))))

(event EventExtra
  (bind _returnvalue (Game|GetPlayerCharacter 0))
  (bind _asbp_arpgcharacter (Utilities|Casting|CastToBP_ARPGCharacter _returnvalue))
  (Variables|/Script/Guaduation_ARPG.ARPGCharacter|SetMoney _asbp_arpgcharacter (+ (Variables|/Script/Guaduation_ARPG.ARPGCharacter|GetMoney _asbp_arpgcharacter) 3.0))
  (Variables|/Script/Guaduation_ARPG.ARPGCharacter|SetExp _asbp_arpgcharacter (+ (Variables|/Script/Guaduation_ARPG.ARPGCharacter|GetExp _asbp_arpgcharacter) 2.0))
  (bind _returnvalue_2 (UserInterface|CreateWidget "/Game/UI/WB_GetInfo.WB_GetInfo_C" 0 (Variables|Default|GetGetInfo)))
  (UserInterface|Viewport|AddtoViewport _returnvalue_2 0))

(fn ConstructionScript)