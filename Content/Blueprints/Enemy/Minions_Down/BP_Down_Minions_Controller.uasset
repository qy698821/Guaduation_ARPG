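; AI controller for the Down Minions enemy that tracks sight of the player through AI Perception.
; A sensed actor tagged Player cancels the forget timer and is written to the Blackboard along with HasSight.
; Any other perception update restarts a LineOfSight-length timer, which clears both Blackboard values on expiry.
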(event OnTargetPerceptionUpdated(AIPerception)
  (params (Actor :type Actor%20Object%20Reference) (Stimulus :type AI%20Stimulus%20Structure))
  (Utilities|IsValid Actor
    (:Is%20Valid
      (Utilities|IsValid (Pawn|GetControlledPawn self)
        (:Is%20Valid
          (if (and (Actor|ActorHasTag Actor "Player") (.bSuccessfullySensed (Utilities|Struct|BreakAIStimulus Stimulus)))
            (Utilities|Time|ClearandInvalidateTimerbyHandle (Variables|Default|GetEnemyTimer))
            (AI|Components|Blackboard|SetValueasObject (Variables|Default|GetBBComponent) (Variables|Default|GetPlayer) Actor)
            (AI|Components|Blackboard|SetValueasBool (Variables|Default|GetBBComponent) (Variables|Default|GetHasSight) true)
            (else
              (bind _returnvalue (Utilities|Time|SetTimerbyEvent (delegate Custom|StartEnemyTimer) (Variables|Default|GetLineOfSight)))
              (Variables|Default|SetEnemyTimer _returnvalue))))))))

(event Custom|StartEnemyTimer
  (AI|Components|Blackboard|SetValueasObject (Variables|Default|GetBBComponent) (Variables|Default|GetPlayer) 0)
  (AI|Components|Blackboard|SetValueasBool (Variables|Default|GetBBComponent) (Variables|Default|GetHasSight) false))

(event EventBeginPlay)

(event EventTick
  (params (DeltaSeconds :type Float%20%28single-precision%29)))

(fn ConstructionScript)