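; Player controller for an action RPG that manages the inventory and in-game widgets and item hotkey input.
; BeginPlay initializes the inventory and creates the in-game widget without adding it to the viewport here.
; Outside the start level, OpenInventory toggles a lazily created inventory widget fed the Inventory array; LoadWidget refreshes both widgets once that widget exists.
; Use1 uses the pickup in the in-game widget's first wrap box slot.
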(event EventBeginPlay
  ;[1 1 1] Create Ingame Widget
  (Class|ARPGPlayerController|InitInventory)
  (bind _returnvalue (UserInterface|CreateWidget "/Game/UI/WB_InGame.WB_InGame_C"))
  (Variables|Default|SetWB_Ingame _returnvalue))

(event EventTick
  (params (DeltaSeconds :type Float%20%28single-precision%29)))

(event EventLoadWidget
  (bind _wb_inventory (Variables|Default|GetWB_Inventory))
  ;[1 1 1] Reload Widget
  (Utilities|IsValid _wb_inventory
    (:Is%20Valid
      (Default|LoadInventory _wb_inventory)
      (Default|LoadWidget (Variables|Default|GetWB_Ingame)))))

(event Input|ActionEvents|InputActionOpenInventory
  (params (Key :type Key%20Structure))
  ;[1 1 1] Open and close inventory system
  (:Pressed
    (if (Variables|Default|GetNotInStartLevel)
      (bind _output_get (Variables|Default|SetIsOpend (not (Variables|Default|GetIsOpend))))
      (if _output_get
        (Utilities|IsValid (Variables|Default|GetWB_Inventory)
          (:Is%20Valid
            _)
          (:Is%20Not%20Valid
            (bind _returnvalue (UserInterface|CreateWidget "/Game/UI/WB_Inventory.WB_Inventory_C" 0 (Variables|Default|GetInventory)))
            (Variables|Default|SetWB_Inventory _returnvalue)))
        (UserInterface|Viewport|AddtoViewport (Variables|Default|GetWB_Inventory) 0)
        (else
          (Widget|RemovefromParent (Variables|Default|GetWB_Inventory)))))))

(event Input|ActionEvents|InputActionUse1
  (params (Key :type Key%20Structure))
  (:Pressed
    (Default|UseItem (.AsC%20Pick%20Up (Utilities|Casting|CastToC_PickUp (Class|PanelWidget|GetChildat (Variables|/Game/UI/WB_InGame.WB_InGame_C|GetWrapBox_98 (Variables|Default|GetWB_Ingame))))))))

(fn ConstructionScript)