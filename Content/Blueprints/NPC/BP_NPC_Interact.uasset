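; Interactable NPC Blueprint that provides a shop and a dialog for the player.
; BeginPlay initializes the shop and makes the player the owner, hiding the Pointer from them; interacting toggles a lazily created WB_Shop, opening also calling the inventory toggle.
; Separate events show and hide a cached WB_Dialog, resetting dialog flags on close.
; DeleteBlockwall destroys any BlockingVolume found at the stored BlockingLocation.
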(event EventBeginPlay
  (Class|NPCInteract|InitShop)
  (Actor|SetOwner (Game|GetPlayerCharacter 0))
  (Class|PrimitiveComponent|SetOwnerNoSee (Variables|Default|GetPointer) true))

(event Collision|EventActorBeginOverlap
  (params (OtherActor :type Actor%20Object%20Reference)))

(event EventTick
  (params (DeltaSeconds :type Float%20%28single-precision%29)))

(event EventObjectInteractBlueprint
  (params (Controller :type Player%20Controller%20Object%20Reference))
  ;[1 1 1] OPEN SHOP
  (bind _asarpgplayer_controller (Utilities|Casting|CastToARPGPlayerController Controller))
  (bind _output_get (Variables|Default|SetIsShopOpend (not (Variables|Default|GetIsShopOpend))))
  (if _output_get
    (Class|ARPGPlayerController|OpenandCloseInventory _asarpgplayer_controller)
    (Utilities|IsValid (Variables|Default|GetWB_Shop)
      (:Is%20Valid
        _)
      (:Is%20Not%20Valid
        (bind _returnvalue (UserInterface|CreateWidget "/Game/UI/UI_NPC/WB_Shop.WB_Shop_C" 0 (Variables|Default|GetShopItem) self))
        (Variables|Default|SetWB_Shop _returnvalue)))
    (UserInterface|Viewport|AddtoViewport (Variables|Default|GetWB_Shop) 0)
    (else
      (Widget|RemovefromParent (Variables|Default|GetWB_Shop)))))

(event EventOpenDialogWidget
  ;[1 1 1] OPEN DIALOG WIDGET
  (Utilities|IsValid (Variables|Default|GetWB_Dialog)
    (:Is%20Valid
      _)
    (:Is%20Not%20Valid
      (bind _returnvalue (UserInterface|CreateWidget "/Game/UI/UI_NPC/WB_Dialog.WB_Dialog_C" 0 self))
      (bind _output_get (Variables|Default|SetWB_Dialog _returnvalue))))
  (if (not (Widget|IsVisible (Variables|Default|GetWB_Dialog)))
    (UserInterface|Viewport|AddtoViewport _output_get 0)))

(event EventCloseDialogWidget
  (bind _wb_dialog (Variables|Default|GetWB_Dialog))
  ;[1 1 1] CLOSE DIALOG WIDGET
  (Variables|Default|SetShouldCloseWidget false)
  (Variables|Default|SetIsEndOfDialog false)
  (if (Widget|IsVisible _wb_dialog)
    (Widget|RemovefromParent _wb_dialog)))

(event EventDeleteBlockwall
  (bind _outactors (Actor|GetAllActorsOfClass "/Script/Engine.BlockingVolume"))
  (for _array_element _outactors
    (if (<= (Math|Vector|Distance(Vector) (Transformation|GetActorLocation _array_element) (Variables|Default|GetBlockingLocation)) 2.0)
      (Actor|DestroyActor _array_element))))

(fn ConstructionScript)